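; Enemy Blueprint that wanders, chases the player on sight and tracks its health on a life bar widget.
; Marche loops AI moves to random reachable points, while PawnSensing switches to chasing, raises walk speed once and resumes wandering after a retriggerable delay.
; Sphere overlap with the player plays an attack montage without applying damage.
; SetLife subtracts damage, updates the widget and destroys the actor when life equals exactly zero.
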(event OnSeePawn(PawnSensing)
  (params (Pawn :type Pawn%20Object%20Reference))
  (if (== Pawn (Variables|Default|GetPlyerRef))
    (Utilities|FlowControl|Sequence
      (:then_0
        (AI|AIMoveTo self "0, 0, 0" (Variables|Default|GetPlyerRef) 5.0 false))
      (:then_1
        (Utilities|FlowControl|RetriggerableDelay 1.0)
        (CallFunction|Marche))
      (:then_2
        (Utilities|FlowControl|DoOnce false
          (:Completed
            (Variables|/Script/Engine.CharacterMovementComponent|SetMaxWalkSpeed (Variables|Character|GetCharacterMovement) 3.5e+02)))))))

(event OnComponentBeginOverlap(Sphere)
  (params (OverlappedComponent :type Primitive%20Component%20Object%20Reference) (OtherActor :type Actor%20Object%20Reference) (OtherComp :type Primitive%20Component%20Object%20Reference) (OtherBodyIndex :type Integer) (bFromSweep :type Boolean) (SweepResult :type Hit%20Result%20Structure%20%28by%20ref%29))
  (if (== OtherActor (Variables|Default|GetPlyerRef))
    (Animation|Montage|PlayMontage (Variables|Character|GetMesh) "/Game/SkeletonCrew/Skeleton_Swordman/Animations/Skeleton_Swordman_Charge_End_Montage.Skeleton_Swordman_Charge_End_Montage")))

(event Custom|Marche
  (AI|AIMoveTo self (.RandomLocation (AI|Navigation|GetRandomReachablePointinRadius (Transformation|GetActorLocation) 1.5e+03 0 0)) 0 5.0 false
    (:OnSuccess
      (CallFunction|Marche))))

(event EventBeginPlay
  (bind _returnvalue (Actor|GetActorOfClass "/Game/Player/BP_ThirdPersonCharacter.BP_ThirdPersonCharacter_C"))
  (Variables|Default|SetPlyerRef _returnvalue)
  (CallFunction|Marche)
  (bind _asui_lif_bar (Utilities|Casting|CastToUI_LifBar (UserInterface|GetUserWidgetObject (Variables|Default|GetWidget))))
  (bind _output_get (Variables|Default|SetAs%20UI%20Lif%20Bar _asui_lif_bar))
  (bind _output_get_2 (Variables|/Game/Enemies/UI_LifBar.UI_LifBar_C|SetLife _output_get (Variables|Default|GetMaxLife)))
  (Variables|/Game/Enemies/UI_LifBar.UI_LifBar_C|SetMax%20Life _output_get _output_get_2))

(fn ConstructionScript
  (Variables|Default|SetCurrentLife (Variables|Default|GetMaxLife)))

(fn SetLife
  (params (Damages :type Float%20%28double-precision%29))
  (bind _output_get (Variables|Default|SetCurrentLife (- (Variables|Default|GetCurrentLife) Damages)))
  (bind _output_get_2 (Variables|/Game/Enemies/UI_LifBar.UI_LifBar_C|SetLife (Variables|Default|GetAs%20UI%20Lif%20Bar) _output_get))
  (if (== _output_get_2 0.0)
    (CallFunction|Die)))

(fn Die
  (Actor|DestroyActor))